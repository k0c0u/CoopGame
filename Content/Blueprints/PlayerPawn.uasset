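; PlayerPawn is a player pawn Blueprint that sets up the on-screen HUD for the local player.
; On BeginPlay, a local-control check gates creating the crosshair and health indicator widgets and adding them to the viewport.
; Tick repeats that check but does nothing.
; An unconnected chain to spawn a rifle, store it as the current weapon and attach it to the mesh's weapon socket never runs.
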(event EventBeginPlay
  (if (Pawn|IsLocallyControlled)
    (Utilities|FlowControl|Sequence
      (:then_0
        (bind _returnvalue (UserInterface|CreateWidget "/Game/UI/WBP_Crosshair.WBP_Crosshair_C"))
        (UserInterface|Viewport|AddtoViewport _returnvalue 0))
      (:then_1
        (bind _returnvalue_2 (UserInterface|CreateWidget "/Game/UI/WBP_HaelthIndicator.WBP_HaelthIndicator_C"))
        (UserInterface|Viewport|AddtoViewport _returnvalue_2 0)))))

(event Collision|EventActorBeginOverlap
  (params (OtherActor :type Actor%20Object%20Reference)))

(event EventTick
  (params (DeltaSeconds :type Float%20%28single-precision%29))
  (if (Pawn|IsLocallyControlled)
    _))

(fn ConstructionScript)